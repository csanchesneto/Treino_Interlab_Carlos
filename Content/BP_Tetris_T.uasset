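; BP_Tetris_T is a Tetris piece, likely the T shape, that falls and can be shifted and rotated.
; While Controle is true, Tick lowers the root a fixed step each frame, independent of delta time.
; MovaPeca and MovaPecaEsq shift it along Y in opposite directions, and GiraPeca pitches it a quarter turn.
; Any actor overlap clears Controle to stop the fall, but the move and rotate events never check that flag.
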(event `self.ReceiveActorBeginOverlap`
  (params (OtherActor :type "Actor Object Reference"))
  (set `self.Controle` false))

(event `MovaPecaEsq`
  (`SceneComponent.K2_AddRelativeLocation` (`self.DefaultSceneRoot`) (0.0 -100.0 0.0) false false))

(event `MovaPeca`
  (`SceneComponent.K2_AddRelativeLocation` (`self.DefaultSceneRoot`) (0.0 100.0 0.0) false false))

(event `self.ReceiveTick`
  (params (DeltaSeconds :type "Float (single-precision)"))
  (if (`self.Controle`)
    (`SceneComponent.K2_AddRelativeLocation` (`self.DefaultSceneRoot`) (0.0 0.0 -1.0) false false)))

(event `GiraPeca`
  (`SceneComponent.K2_AddLocalTransform` (`self.DefaultSceneRoot`) (`KismetMathLibrary.MakeTransform` (0.0 0.0 0.0) (`KismetMathLibrary.MakeRotator` 0.0 90.0)) false false))

(fn `UserConstructionScript`)